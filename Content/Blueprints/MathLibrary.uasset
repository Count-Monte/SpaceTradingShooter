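; Blueprint math library of helpers for large-scale space positioning and aiming.
; It converts between Unreal units and kilometers, compares IntVectors, and combines local positions with the world origin location to give integer or precise galaxy positions, or subtracts it for local offsets.
; TargetLead feeds positions and forward-speed velocities of shooter and target into CalculateTargetLead.
; UniformUnitDiscDistribution returns the cosine and sine of random angles.
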(fn Equal(IntVector)
  (params (Param1 :type Int%20Vector%20Structure%20%28by%20ref%29) (Param2 :type Int%20Vector%20Structure%20%28by%20ref%29))
  (bind (_x _y _z) (Utilities|Struct|BreakIntVector Param1))
  (bind (_x_2 _y_2 _z_2) (Utilities|Struct|BreakIntVector Param2))
  (return (Math|Boolean|ANDBoolean (== _x _x_2) (== _y _y_2) (== _z _z_2))))

(fn NotEqual(IntVector)
  (params (Param%201 :type Int%20Vector%20Structure%20%28by%20ref%29) (Param%202 :type Int%20Vector%20Structure%20%28by%20ref%29))
  (return (not (Math|IntVector|Equal(IntVector) Param%201 Param%202 (LocalVariables|Get__WorldContext)))))

(fn KiloMeterstoUU
  (params (Kilometers :type Vector))
  (bind (_x _y _z) (Math|Vector|BreakVector Kilometers))
  (return (Math|Vector|MakeVector (Class|CPPMathLib|KiloMeterstoUU _x) (Class|CPPMathLib|KiloMeterstoUU _y) (Class|CPPMathLib|KiloMeterstoUU _z))))

(fn UUtoKiloMeters
  (params (Vector :type Int%20Vector%20Structure))
  (bind (_x _y _z) (Utilities|Struct|BreakIntVector Vector))
  (return (Utilities|Struct|MakeIntVector (/ (/ _x 1000) 1000) (/ (/ _y 1000) 1000) (/ (/ _z 1000) 1000))))

(fn GetGalaxyPosition
  (params (LocalPositon :type Vector))
  (bind (_x _y _z) (Math|Vector|BreakVector LocalPositon))
  (bind ___worldcontext (LocalVariables|Get__WorldContext))
  (bind _returnvalue (Class|GameplayStatics|GetWorldOriginLocation ___worldcontext))
  (bind (_x_2 _y_2 _z_2) (Utilities|Struct|BreakIntVector _returnvalue))
  (return (Utilities|Struct|MakeIntVector (+ (Math|Float|Floor (Class|CPPMathLib|UUtoKiloMeters _x)) (Math|Integer|UUtoKiloMeters(Integer) _x_2 ___worldcontext)) (+ (Math|Float|Floor (Class|CPPMathLib|UUtoKiloMeters _y)) (Math|Integer|UUtoKiloMeters(Integer) _y_2 ___worldcontext)) (+ (Math|Float|Floor (Class|CPPMathLib|UUtoKiloMeters _z)) (Math|Integer|UUtoKiloMeters(Integer) _z_2 ___worldcontext)))))

(fn UUtoKiloMeters(Integer)
  (params (Int :type Integer))
  (return (/ (/ Int 1000) 1000)))

(fn KiloMeterstoUU(Integer)
  (params (Kilo :type Integer))
  (return (* (* Kilo 1000) 1000)))

(fn GetGalaxyPosition(Precise)
  (params (LocalPositon :type Vector))
  (bind (_x _y _z) (Math|Vector|BreakVector LocalPositon))
  (bind ___worldcontext (LocalVariables|Get__WorldContext))
  (bind _returnvalue (Class|GameplayStatics|GetWorldOriginLocation ___worldcontext))
  (bind (_x_2 _y_2 _z_2) (Utilities|Struct|BreakIntVector _returnvalue))
  (return (Math|Vector|MakeVector (+ (Class|CPPMathLib|UUtoKiloMeters _x) (Class|CPPMathLib|UUtoKiloMeters (Math|Conversions|ToFloat(Integer) _x_2))) (+ (Class|CPPMathLib|UUtoKiloMeters _y) (Class|CPPMathLib|UUtoKiloMeters (Math|Conversions|ToFloat(Integer) _y_2))) (+ (Class|CPPMathLib|UUtoKiloMeters _z) (Class|CPPMathLib|UUtoKiloMeters (Math|Conversions|ToFloat(Integer) _z_2))))))

(fn GetLocalOffset
  (params (WorldPosition :type Vector))
  (bind (_x _y _z) (Math|Vector|BreakVector WorldPosition))
  (bind ___worldcontext (LocalVariables|Get__WorldContext))
  (bind _returnvalue (Class|GameplayStatics|GetWorldOriginLocation ___worldcontext))
  (bind (_x_2 _y_2 _z_2) (Utilities|Struct|BreakIntVector _returnvalue))
  (return (Math|Vector|MakeVector (- _x (Math|Conversions|ToFloat(Integer) _x_2)) (- _y (Math|Conversions|ToFloat(Integer) _y_2)) (- _z (Math|Conversions|ToFloat(Integer) _z_2)))))

(fn UniformUnitDiscDistribution
  (bind _returnvalue (Math|Float|MultiplybyPi 2.0))
  (bind _returnvalue_2 (Math|Random|RandomFloatinRange 0.0 _returnvalue))
  (return (Math|Trig|Cos(Radians) _returnvalue_2) (Math|Trig|Sin(Radians) _returnvalue_2)))

(fn TargetLead
  (params (Shooter :type Ship%20Object%20Reference) (Target :type Ship%20Object%20Reference) (ShootSpeed :type Float%20%28single-precision%29))
  (return (Class|CPPMathLib|CalculateTargetLead (Transformation|GetActorLocation Shooter) (* (Transformation|GetActorForwardVector Shooter) (Variables|/Game/Blueprints/Ships/Ship.Ship_C|GetCurrent%20Forward%20speed Shooter)) ShootSpeed (Transformation|GetActorLocation Target) (* (Transformation|GetActorForwardVector Target) (Variables|/Game/Blueprints/Ships/Ship.Ship_C|GetCurrent%20Forward%20speed Target)))))