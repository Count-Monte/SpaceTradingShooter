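; Bullet projectile that damages ships it hits and expires after a fixed lifespan if it hits nothing.
; On hit it passes any Ship other than its instigator to BulletHit, then destroys itself.
; BulletHit spawns an impact emitter aligned to the surface normal and scaled to the bullet's sphere.
; It applies damage with a bullet damage type, crediting the firing ship's controller when that ship is valid.
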(event EventBeginPlay
  (Actor|SetLifeSpan 1e+01))

(event EventTick
  (params (DeltaSeconds :type Float%20%28single-precision%29)))

(event Collision|EventHit
  (params (MyComp :type Primitive%20Component%20Object%20Reference) (Other :type Actor%20Object%20Reference) (OtherComp :type Primitive%20Component%20Object%20Reference) (bSelfMoved :type Boolean) (HitLocation :type Vector :default "0, 0, 0") (HitNormal :type Vector :default "0, 0, 0") (NormalImpulse :type Vector :default "0, 0, 0") (Hit :type Hit%20Result%20Structure%20%28by%20ref%29))
  (bind _returnvalue (Game|GetInstigator))
  (if (!= Other _returnvalue)
    (bind _asship (Utilities|Casting|CastToShip Other)
      (:then
        (bind _asship_2 (Utilities|Casting|CastToShip _returnvalue)
          (:then
            _)
          (:CastFailed
            _))
        (CallFunction|BulletHit _asship (select (Utilities|IsValid _returnvalue) _asship_2 0) HitLocation HitNormal))
      (:CastFailed
        _)))
  (Actor|DestroyActor))

(fn ConstructionScript)

(fn BulletHit
  (params (OtherShip :type Ship%20Object%20Reference) (MyShip :type Ship%20Object%20Reference) (HitLocation :type Vector) (HitNormal :type Vector))
  (bind _self self)
  (bind _damage (Variables|Default|GetDamage))
  (Effects|SpawnEmitteratLocation self (Variables|Default|GetHitPS) HitLocation (Math|Conversions|RotationFromXVector HitNormal) (Transformation|GetWorldScale (Variables|Default|GetSphere)))
  (Utilities|IsValid MyShip
    (:Is%20Valid
      (Game|Damage|ApplyDamage OtherShip _damage (Pawn|GetController MyShip) _self "/Game/Blueprints/Projectiles/Bullet_DT.Bullet_DT_C"))
    (:Is%20Not%20Valid
      (Game|Damage|ApplyDamage OtherShip _damage 0 _self "/Game/Blueprints/Projectiles/Bullet_DT.Bullet_DT_C"))))