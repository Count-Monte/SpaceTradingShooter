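; TriFighter is a ship Blueprint that starts play fitted with laser weapons and a mining laser.
; On BeginPlay it calls the parent logic, registers its two weapon slots and one mining laser slot, then assigns laser weapon equipment to both weapon slots and mining laser equipment to the third.
; It has no active tick or overlap logic, and its construction script only calls the parent.
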(event EventBeginPlay
  (bind _mininglaserslot (Variables|Default|GetMiningLaserSlot))
  (bind _weaponslot1 (Variables|Default|GetWeaponSlot1))
  (bind _weaponslot2 (Variables|Default|GetWeaponSlot2))
  (|CallParentFunction)
  (CallFunction|RegisterEquipmentSlots (Utilities|Array|MakeArray _weaponslot1 _weaponslot2 _mininglaserslot))
  (Default|SetEquipment _weaponslot1 "/Game/Blueprints/Equipment/LaserWeaponEquipment.LaserWeaponEquipment_C")
  (Default|SetEquipment _weaponslot2 "/Game/Blueprints/Equipment/LaserWeaponEquipment.LaserWeaponEquipment_C")
  (Default|SetEquipment _mininglaserslot "/Game/Blueprints/Equipment/MiningLaserEquipment.MiningLaserEquipment_C"))

(event Collision|EventActorBeginOverlap
  (params (OtherActor :type Actor%20Object%20Reference)))

(event EventTick
  (params (DeltaSeconds :type Float%20%28single-precision%29))
  (|CallParentFunction DeltaSeconds) ; This node is disabled and will not be called.\nDrag off pins to build functionality.
)

(fn ConstructionScript
  (|CallParentFunction))