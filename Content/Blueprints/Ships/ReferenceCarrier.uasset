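; ReferenceCarrier is a carrier ship Blueprint that carries eight turrets as child actor components.
; On BeginPlay it gathers the turret components into an array, casts each child actor to BP_ShipTurret and initializes it with the carrier as argument.
; The construction script assigns an arrow component as the gun barrel, while Tick and construction otherwise defer to the parent class.
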(event EventBeginPlay
  (|CallParentFunction)
  (bind _output_get (Variables|Default|SetTurrets (Utilities|Array|MakeArray (Variables|Default|GetBP_Turret) (Variables|Default|GetBP_Turret1) (Variables|Default|GetBP_Turret2) (Variables|Default|GetBP_Turret3) (Variables|Default|GetBP_Turret4) (Variables|Default|GetBP_Turret5) (Variables|Default|GetBP_Turret6) (Variables|Default|GetBP_Turret7))))
  (for _array_element _output_get
    (bind _asbp_ship_turret (Utilities|Casting|CastToBP_ShipTurret (Variables|/Script/Engine.ChildActorComponent|GetChildActor _array_element)))
    (Default|Init _asbp_ship_turret self)))

(event Collision|EventActorBeginOverlap
  (params (OtherActor :type Actor%20Object%20Reference))
  (|CallParentFunction OtherActor) ; This node is disabled and will not be called.\nDrag off pins to build functionality.
)

(event EventTick
  (params (DeltaSeconds :type Float%20%28single-precision%29))
  (|CallParentFunction DeltaSeconds))

(fn ConstructionScript
  (Variables|Default|SetGun%20Barrel (Variables|Default|GetArrow))
  (|CallParentFunction))