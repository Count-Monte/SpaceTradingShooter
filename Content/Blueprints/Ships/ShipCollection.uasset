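; ShipCollection is a container actor that groups ships and drives their per-frame update.
; Each frame it loops over its Ships array and calls Tick on every valid ship with the frame's delta time.
; AddShip appends a ship and attaches it to the collection, keeping relative transforms.
; RemoveShip takes a ship out of the array and returns the result, without detaching it.
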(event EventBeginPlay)

(event Collision|EventActorBeginOverlap
  (params (OtherActor :type Actor%20Object%20Reference)))

(event EventTick
  (params (DeltaSeconds :type Float%20%28single-precision%29))
  (for _array_element (Variables|Default|GetShips)
    (Utilities|IsValid _array_element
      (:Is%20Valid
        (Default|Tick _array_element DeltaSeconds)))))

(fn ConstructionScript)

(fn AddShip
  (params (Ship :type Ship%20Object%20Reference))
  (Utilities|Array|Add (Variables|Default|GetShips) Ship)
  (Transformation|AttachActorToActor Ship self "None" "KeepRelative" "KeepRelative" "KeepRelative" true))

(fn RemoveShip
  (params (Ship :type Ship%20Object%20Reference))
  (bind _returnvalue (Utilities|Array|RemoveItem (Variables|Default|GetShips) Ship))
  (return _returnvalue))