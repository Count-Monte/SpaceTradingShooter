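; Space shooter game state Blueprint that sets up the playable star system and tracks whether the map is open.
; StarSystemLoaded stores the systems in the globals instance, spawns a scaled WarpableStarsystem and loads the first entry into it.
; It then creates the player and attaches the star system to the returned actor.
; ToggleMap alternates open and close map calls; the GalaxyMapManager spawn is left disconnected.
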(fn ConstructionScript)

(fn ToggleMap
  (if (Variables|Default|GetMapOpen)
    (Default|CallCloseMap)
    (else
      (Default|CallOpenMap)))
  (Variables|Default|SetMapOpen (not (Variables|Default|GetMapOpen))))

(fn StarSystemLoaded
  (params (InStarSystems :type Array%20of%20Star%20System%20Info%20Structures))
  (bind _globals (CallFunction|GetGlobalsInstance))
  (bind _output_get (Variables|/Game/Blueprints/Globals.Globals_C|SetStarSystems _globals InStarSystems))
  (bind _output_get_2 (Variables|Default|SetStarSystems _output_get))
  (bind _returnvalue (Game|SpawnActorfromClass "/Game/Blueprints/World/StarSystem/System/WarpableStarsystem.WarpableStarsystem_C" (Math|Transform|MakeTransform "0, 0, 0" "0, 0, 0" (Math|Conversions|ToVector(Float) (Variables|Default|GetStarSystemSCale))) "AlwaysSpawn" 0 0))
  (bind _output_get_3 (Variables|Default|SetStarSystem _returnvalue))
  (bind _output_get_4 (Variables|/Game/Blueprints/Globals.Globals_C|SetWarpableStarSystem _globals _output_get_3))
  (Default|LoadStarSystem _output_get_4 (Utilities|Array|Get(acopy) _output_get_2))
  (bind _asspace_shooter_player (Utilities|Casting|CastToSpaceShooterPlayer (Game|GetPlayerController 0)))
  (bind _playership (Default|CreatePlayer _asspace_shooter_player "1.000000, 0, 0"))
  (Transformation|AttachActorToActor _returnvalue _playership "None" "KeepRelative" "KeepRelative" "KeepRelative" true))