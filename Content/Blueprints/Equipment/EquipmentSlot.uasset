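; Equipment slot actor that holds equipment matching its accepted type and size.
; SetEquipment checks the class defaults of the requested class, then calls ClearEquipment, spawns the new actor, attaches it to the slot and initializes it with the instigator.
; ClearEquipment destroys the actor in the Equipment variable if valid, though SetEquipment does not store the spawned actor there.
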(event EventBeginPlay)

(event Collision|EventActorBeginOverlap
  (params (OtherActor :type Actor%20Object%20Reference)))

(event EventTick
  (params (DeltaSeconds :type Float%20%28single-precision%29)))

(fn ConstructionScript)

(fn SetEquipment
  (params (Equipment :type Equipment%20Class%20Reference) (Instigator :type Ship%20Object%20Reference))
  (bind (_equipmenttype _equipmentsize) (Utilities|GetClassDefaults Equipment))
  (if (and (== _equipmenttype (Variables|Default|GetAcceptedEquipmentType)) (== _equipmentsize (Variables|Default|GetAcceptedEquipmentSize)))
    (CallFunction|ClearEquipment)
    (bind _returnvalue (Game|SpawnActorfromClass Equipment (Math|Transform|MakeTransform "0, 0, 0" "0, 0, 0" "1,1,1") "AlwaysSpawn" 0 Instigator))
    (Transformation|AttachActorToActor _returnvalue self "None" "KeepRelative" "KeepRelative" "KeepRelative" true)
    (Default|InitEquipment _returnvalue Instigator)))

(fn ClearEquipment
  (bind _equipment (Variables|Default|GetEquipment))
  (Utilities|IsValid _equipment
    (:Is%20Valid
      (Actor|DestroyActor _equipment))))