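; Automatic weapon equipment that fires physics-driven projectiles at a capped fire rate, triggered by PrimaryAction or a direct Fire call.
; InitWeapon sets the muzzle component, and Fire checks a timestamp-based cooldown before spawning the projectile with damage and instigator, then launching it with a velocity-change impulse on its Sphere.
; RelativeSpeed adds to projectile speed and offsets the spawn point forward by one frame of travel; PrimaryAction passes zero.
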(event EventBeginPlay
  (|CallParentFunction) ; This node is disabled and will not be called.\nDrag off pins to build functionality.
)

(event Collision|EventActorBeginOverlap
  (params (OtherActor :type Actor%20Object%20Reference))
  (|CallParentFunction OtherActor) ; This node is disabled and will not be called.\nDrag off pins to build functionality.
)

(event EventTick
  (params (DeltaSeconds :type Float%20%28single-precision%29))
  (|CallParentFunction DeltaSeconds) ; This node is disabled and will not be called.\nDrag off pins to build functionality.
)

(event EventPrimaryAction
  (CallFunction|Fire 0.0))

(fn ConstructionScript
  (|CallParentFunction))

(fn Fire
  (params (RelativeSpeed :type Float%20%28single-precision%29) (Instigator :type Ship%20Object%20Reference))
  (bind _cooldown (CallFunction|HasCooldown))
  (bind _firinglocation (Variables|Default|GetFiringLocation))
  (bind _returnvalue (not _cooldown))
  (bind _returnvalue_2 (Math|Vector|GetForwardVector _firinglocation))
  (if _returnvalue
    (Utilities|FlowControl|Sequence
      (:then_0
        (Variables|Default|SetLastProjectileFireTime (Utilities|Time|GetGameTimeinSeconds))
        (bind _returnvalue_3 (Game|SpawnActorfromClass (Variables|Default|GetProjectileType) (Math|Transform|MakeTransform (+ (Transformation|GetWorldLocation _firinglocation) (* _returnvalue_2 (* RelativeSpeed (Utilities|Time|GetWorldDeltaSeconds)))) (Math|Rotator|MakeRotfromX _returnvalue_2) "1,1,1") "Undefined" 0 (Variables|Default|GetProjectileDamage) Instigator))
        (Utilities|IsValid _returnvalue_3
          (:Is%20Valid
            (Physics|AddImpulse (Variables|/Game/Blueprints/Projectiles/Bullet.Bullet_C|GetSphere _returnvalue_3) (* _returnvalue_2 (+ RelativeSpeed (Variables|Default|GetProjectileSpeed))) "None" true))))
      (:then_1
        (return _returnvalue)))))

(fn HasCooldown
  (return (<= (Utilities|Time|GetGameTimeinSeconds) (+ (Variables|Default|GetLastProjectileFireTime) (/ 1.0 (Variables|Default|GetFireRate))))))

(fn InitWeapon
  (params (BulletSpawnLocation :type Arrow%20Component%20Object%20Reference))
  (Variables|Default|SetFiringLocation BulletSpawnLocation))