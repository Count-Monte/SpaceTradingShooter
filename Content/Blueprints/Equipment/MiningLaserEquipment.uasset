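; Mining laser equipment Blueprint that mines individual asteroids from an AsteroidBelt when its primary action fires.
; BeginPlay registers the Arrow component as the firing location, from which Fire draws a debug line and runs a Visibility line trace out to the beam's maximum distance.
; On a hit, TargetHit passes the struck hierarchical instanced mesh component and instance index to the belt's AsteroidMined, which handles the mining.
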(event EventBeginPlay
  (|CallParentFunction)
  (CallFunction|InitBeamEquipment (Variables|Default|GetArrow)))

(event Collision|EventActorBeginOverlap
  (params (OtherActor :type Actor%20Object%20Reference))
  (|CallParentFunction OtherActor) ; This node is disabled and will not be called.\nDrag off pins to build functionality.
)

(event EventTick
  (params (DeltaSeconds :type Float%20%28single-precision%29))
  (|CallParentFunction DeltaSeconds) ; This node is disabled and will not be called.\nDrag off pins to build functionality.
)

(event EventPrimaryAction
  (CallFunction|Fire))

(fn ConstructionScript
  (|CallParentFunction))

(fn Fire
  (bind _firinglocation (Variables|Default|GetFiringLocation))
  (bind _beammaxdistance (Variables|Default|GetBeamMaxDistance))
  (bind _returnvalue (Math|Vector|GetForwardVector _firinglocation))
  (bind _returnvalue_2 (Transformation|GetWorldLocation _firinglocation))
  (bind _returnvalue_3 (* _returnvalue _beammaxdistance))
  (bind _returnvalue_4 (+ _returnvalue_3 _returnvalue_2))
  (Rendering|Debug|DrawDebugLine _returnvalue_2 _returnvalue_4 "(R=1.000000,G=0.000000,B=0.007021,A=1.000000)" 0.0 0.0)
  (bind (_outhit _returnvalue_5) (Collision|LineTraceByChannel _returnvalue_2 _returnvalue_4 "TraceTypeQuery1" false 0 "None"))
  (if _returnvalue_5
    (CallFunction|TargetHit _outhit)))

(fn InitBeamEquipment
  (params (FiringLocation :type Arrow%20Component%20Object%20Reference))
  (Variables|Default|SetFiringLocation FiringLocation))

(fn TargetHit
  (params (Hit :type Hit%20Result%20Structure))
  (bind (_bblockinghit _binitialoverlap _time _distance _location _impactpoint _normal _impactnormal _physmat _hitactor _hitcomponent _hitbonename _hititem) (Collision|BreakHitResult Hit))
  ;[1 1 1] Example code for mining asteroids
  (bind _asasteroid_belt (Utilities|Casting|CastToAsteroidBelt _hitactor))
  (bind _ashierarchical_instanced_static_mesh_component (Utilities|Casting|CastToHierarchicalInstancedStaticMeshComponent _hitcomponent))
  (Default|AsteroidMined _asasteroid_belt _ashierarchical_instanced_static_mesh_component _hititem))