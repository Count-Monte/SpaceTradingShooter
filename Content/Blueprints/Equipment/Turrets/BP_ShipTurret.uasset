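; BP_ShipTurret is a twin-barrel turret that mounts on a ship and delegates its behaviour to an AITurret component.
; Its Init stores the owning ship, then passes the base, barrel container, both shoot locations, targeting range and turn speed to AITurret.
; The turret targets ships, scales itself from the scene's world scale, and runs with debug enabled.
; The event graph holds no active logic.
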(event EventBeginPlay)

(event Collision|EventActorBeginOverlap
  (params (OtherActor :type Actor%20Object%20Reference)))

(event EventTick
  (params (DeltaSeconds :type Float%20%28single-precision%29)))

(fn ConstructionScript)

(fn Init
  (params (OwningShip :type Ship%20Object%20Reference))
  (bind _output_get (Variables|Default|SetOwningShip OwningShip))
  (Default|Init (Variables|Default|GetAITurret) (Variables|Default|GetTurretBase) (Variables|Default|GetBarrelContainer) (Utilities|Array|MakeArray (Variables|Default|GetBarrel1ShootLocation) (Variables|Default|GetBarrel2ShootLocation)) (Variables|Default|GetTargetingRange) "/Game/Blueprints/Ships/Ship.Ship_C" true 2e+02 _output_get (/ (.X (Math|Vector|BreakVector (Transformation|GetWorldScale (Variables|Default|GetScene)))) 2.0)))