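; Ship equipment slot component that holds one spawned equipment actor for its owning ship.
; SetEquipment checks the class defaults against the slot's accepted type and size, then destroys any current equipment and spawns, attaches and initializes the replacement.
; Init stores the owning ship, which becomes the equipment's instigator.
; PrimaryAction forwards to the equipment only if it is a ControllableEquipment.
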(event EventBeginPlay)

(event EventTick
  (params (DeltaSeconds :type Float%20%28single-precision%29)))

(fn SetEquipment
  (params (Equipment :type Equipment%20Class%20Reference))
  (bind _output_get (Variables|Default|SetEquipmentClass Equipment))
  (if (and (== (.EquipmentType (Utilities|GetClassDefaults _output_get)) (Variables|Default|GetAcceptedEquipmentType)) (== (.EquipmentSize (Utilities|GetClassDefaults _output_get)) (Variables|Default|GetAcceptedEquipmentSize)))
    (CallFunction|ClearEquipment)
    (bind _returnvalue (Game|SpawnActorfromClass _output_get (Math|Transform|MakeTransform "0, 0, 0" "0, 0, 0" "1,1,1") "AlwaysSpawn" 0 (Variables|Default|GetOwningShip)))
    (Transformation|AttachComponentToComponent _returnvalue self "None" "KeepRelative" "KeepRelative" "KeepRelative" true)
    (bind _output_get_2 (Variables|Default|SetEquipment _returnvalue))
    (Default|InitEquipment _output_get_2 (Variables|Default|GetOwningShip))))

(fn ClearEquipment
  (bind _equipment (Variables|Default|GetEquipment))
  (Utilities|IsValid _equipment
    (:Is%20Valid
      (Actor|DestroyActor _equipment))))

(fn Init
  (params (Ship :type Ship%20Object%20Reference))
  (Variables|Default|SetOwningShip Ship))

(fn HasEquipment
  (return (Utilities|IsValid (Variables|Default|GetEquipment))))

(fn PrimaryAction
  (bind _hasequipment (CallFunction|HasEquipment))
  (if _hasequipment
    (bind _ascontrollable_equipment (Utilities|Casting|CastToControllableEquipment (Variables|Default|GetEquipment)))
    (Default|PrimaryAction _ascontrollable_equipment)))