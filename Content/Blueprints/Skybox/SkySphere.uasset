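; SkySphere is a skybox actor that follows the player's Ship through the world.
; On BeginPlay its Scene component switches to absolute rotation and scale, so it inherits only location from a parent.
; Each Tick it checks the player pawn and, when that is a Ship other than the stored one, stores it and attaches itself to it with relative rules.
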(event EventBeginPlay
  (Transformation|SetAbsolute (Variables|Default|GetScene) false true true))

(event Collision|EventActorBeginOverlap
  (params (OtherActor :type Actor%20Object%20Reference)))

(event EventTick
  (params (DeltaSeconds :type Float%20%28single-precision%29))
  (bind _returnvalue (Game|Player|GetPlayerPawn 0))
  (Utilities|IsValid _returnvalue
    (:Is%20Valid
      (bind _asship (Utilities|Casting|CastToShip _returnvalue))
      (if (!= _returnvalue (Variables|Default|GetAttachedTo))
        (bind _output_get (Variables|Default|SetAttachedTo _asship))
        (Transformation|AttachActorToActor _output_get "None" "KeepRelative" "KeepRelative" "KeepRelative" false)))))

(fn ConstructionScript)