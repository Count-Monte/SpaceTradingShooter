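; Behavior tree task that makes an AI Ship assault the blackboard Target Ship for a blackboard-set duration, then succeeds.
; Each tick converts the direction to the target into local space to drive thrust, strafe and vertical movement, without steering rotation.
; It fires when facing the target closely; the intended range check measures a unit vector, so it always passes.
; It fails if either Ship cast fails.
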(event EventReceiveExecuteAI
  (params (OwnerController :type AI%20Controller%20Object%20Reference) (ControlledPawn :type Pawn%20Object%20Reference))
  (if (not (Variables|Default|GetActive))
    (Variables|Default|SetActive true)
    (Variables|Default|SetAssaultEndDuration (+ (Utilities|Time|GetGameTimeinSeconds) (Class|BTFunctionLibrary|GetBlackboardValueasFloat (Variables|Default|GetAssaultDuration))))))

(event EventReceiveAbortAI
  (params (OwnerController :type AI%20Controller%20Object%20Reference) (ControlledPawn :type Pawn%20Object%20Reference))
  ;[1 1 1] Handle abort
  (Variables|Default|SetActive false)
  (Class|BTTaskBlueprintBase|FinishAbort))

(event EventReceiveTickAI
  (params (OwnerController :type AI%20Controller%20Object%20Reference) (ControlledPawn :type Pawn%20Object%20Reference) (DeltaSeconds :type Float%20%28single-precision%29))
  (if (< (Variables|Default|GetAssaultEndDuration) (Utilities|Time|GetGameTimeinSeconds))
    (Variables|Default|SetActive false)
    (AI|BehaviorTree|FinishExecute true)
    (else
      (bind _asship (Utilities|Casting|CastToShip ControlledPawn)
        (:then
          (bind _asship_2 (Utilities|Casting|CastToShip (Class|BTFunctionLibrary|GetBlackboardValueasObject (Variables|Default|GetTarget)))
            (:then
              (Utilities|FlowControl|Sequence
                (:then_0
                  ;[1 1 1] Move ship after assult direction
                  (Utilities|FlowControl|Sequence
                    (:then_0
                      (Default|Thrust _asship (.X (Math|Vector|BreakVector (Math|Vector|UnrotateVector (Math|Vector|GetUnitDirection(Vector) (Transformation|GetActorLocation _asship) (Transformation|GetActorLocation _asship_2)) (Transformation|GetActorRotation _asship))))))
                    (:then_1
                      (Default|MoveUp _asship (.Z (Math|Vector|BreakVector (Math|Vector|UnrotateVector (Math|Vector|GetUnitDirection(Vector) (Transformation|GetActorLocation _asship) (Transformation|GetActorLocation _asship_2)) (Transformation|GetActorRotation _asship)))) 1.0))
                    (:then_2
                      (Default|MoveRight _asship (.Y (Math|Vector|BreakVector (Math|Vector|UnrotateVector (Math|Vector|GetUnitDirection(Vector) (Transformation|GetActorLocation _asship) (Transformation|GetActorLocation _asship_2)) (Transformation|GetActorRotation _asship))))))))
                (:then_1
                  ;[1 1 1] Should Fire
                  (if (and (> (Math|Vector|DotProduct (Math|Vector|GetUnitDirection(Vector) (Transformation|GetActorLocation _asship) (Transformation|GetActorLocation _asship_2)) (Transformation|GetActorForwardVector _asship)) 0.95) (< (Math|Vector|VectorLength (Math|Vector|GetUnitDirection(Vector) (Transformation|GetActorLocation _asship) (Transformation|GetActorLocation _asship_2))) 5e+03))
                    (Default|Fire _asship)))))
            (:CastFailed
              (Variables|Default|SetActive false :!label _label)
              (AI|BehaviorTree|FinishExecute false))))
        (:CastFailed
          (goto _label))))))