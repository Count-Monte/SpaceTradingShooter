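; Behavior tree task that lets an AI-controlled Ship acquire a target from its sensor.
; On execute it casts the pawn to Ship, takes the first actor in sensor range and writes it to the Target blackboard key with FoundTarget set true, then succeeds.
; If the cast fails or nothing is in range, it sets FoundTarget false and fails, leaving Target unchanged.
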(event EventReceiveExecuteAI
  (params (OwnerController :type AI%20Controller%20Object%20Reference) (ControlledPawn :type Pawn%20Object%20Reference))
  (bind _foundtarget (Variables|Default|GetFoundTarget))
  (bind _asship (Utilities|Casting|CastToShip ControlledPawn)
    (:then
      (bind _ships (Default|GetActorsinRangeOfSensor _asship))
      (if (> (Utilities|Array|Length _ships) 0)
        (Class|BTFunctionLibrary|SetBlackboardValueasBool _foundtarget true)
        (Class|BTFunctionLibrary|SetBlackboardValueasObject (Variables|Default|GetTarget) (Utilities|Array|Get(acopy) _ships))
        (AI|BehaviorTree|FinishExecute true)
        (else
          (Class|BTFunctionLibrary|SetBlackboardValueasBool _foundtarget false :!label _label)
          (AI|BehaviorTree|FinishExecute false))))
    (:CastFailed
      (goto _label))))