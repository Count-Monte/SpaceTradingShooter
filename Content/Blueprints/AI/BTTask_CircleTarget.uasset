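; Behavior tree task that makes an AI-controlled Ship circle its blackboard Target ship for a blackboard-defined duration.
; Each tick rotates the direction to the target about world Z, blending from head-on when far to perpendicular within OrbitRange.
; That vector, converted into the ship's local space, drives Thrust, MoveRight and MoveUp.
; It succeeds when time expires and fails if either object is not a Ship.
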(event EventReceiveAbortAI
  (params (OwnerController :type AI%20Controller%20Object%20Reference) (ControlledPawn :type Pawn%20Object%20Reference))
  ;[1 1 1] Handle abort
  (Variables|Default|SetTaskActive false)
  (Class|BTTaskBlueprintBase|FinishAbort))

(event EventReceiveTickAI
  (params (OwnerController :type AI%20Controller%20Object%20Reference) (ControlledPawn :type Pawn%20Object%20Reference) (DeltaSeconds :type Float%20%28single-precision%29))
  (bind _orbitrange (Variables|Default|GetOrbitRange))
  ;[1 1 1] Stop execution if time was reached
  (if (< (Variables|Default|GetTaskEndTime) (Utilities|Time|GetGameTimeinSeconds))
    (Variables|Default|SetTaskActive false)
    (AI|BehaviorTree|FinishExecute true)
    (else
      ;[1 1 1] Verify that controlled pawn and target objects are ships. Otherwise fail task.
      (bind _asship (Utilities|Casting|CastToShip ControlledPawn)
        (:then
          (bind _asship_2 (Utilities|Casting|CastToShip (Class|BTFunctionLibrary|GetBlackboardValueasObject (Variables|Default|GetTarget)))
            (:then
              ;[1 1 1] Move ship after circle direction
              (Utilities|FlowControl|Sequence
                (:then_0
                  (Default|Thrust _asship (.X (Math|Vector|BreakVector (Math|Vector|UnrotateVector (Math|Vector|RotateVectorAroundAxis (Math|Vector|GetUnitDirection(Vector) (Transformation|GetActorLocation _asship) (Transformation|GetActorLocation _asship_2)) (Math|Float|Lerp 9e+01 0.0 (Math|Float|Clamp(Float) (/ (- (Math|Vector|Distance(Vector) (Transformation|GetActorLocation _asship) (Transformation|GetActorLocation _asship_2)) _orbitrange) (+ _orbitrange 5e+02)))) "0.000000, 0,1.000000") (Transformation|GetActorRotation _asship))))))
                (:then_1
                  (Default|MoveUp _asship (.Z (Math|Vector|BreakVector (Math|Vector|UnrotateVector (Math|Vector|RotateVectorAroundAxis (Math|Vector|GetUnitDirection(Vector) (Transformation|GetActorLocation _asship) (Transformation|GetActorLocation _asship_2)) (Math|Float|Lerp 9e+01 0.0 (Math|Float|Clamp(Float) (/ (- (Math|Vector|Distance(Vector) (Transformation|GetActorLocation _asship) (Transformation|GetActorLocation _asship_2)) _orbitrange) (+ _orbitrange 5e+02)))) "0.000000, 0,1.000000") (Transformation|GetActorRotation _asship)))) 1.0))
                (:then_2
                  (Default|MoveRight _asship (.Y (Math|Vector|BreakVector (Math|Vector|UnrotateVector (Math|Vector|RotateVectorAroundAxis (Math|Vector|GetUnitDirection(Vector) (Transformation|GetActorLocation _asship) (Transformation|GetActorLocation _asship_2)) (Math|Float|Lerp 9e+01 0.0 (Math|Float|Clamp(Float) (/ (- (Math|Vector|Distance(Vector) (Transformation|GetActorLocation _asship) (Transformation|GetActorLocation _asship_2)) _orbitrange) (+ _orbitrange 5e+02)))) "0.000000, 0,1.000000") (Transformation|GetActorRotation _asship))))))))
            (:CastFailed
              (Variables|Default|SetTaskActive false :!label _label)
              (AI|BehaviorTree|FinishExecute false))))
        (:CastFailed
          (goto _label))))))

(event EventReceiveExecuteAI
  (params (OwnerController :type AI%20Controller%20Object%20Reference) (ControlledPawn :type Pawn%20Object%20Reference))
  ;[1 1 1] Setup first time execution of task
  (if (not (Variables|Default|GetTaskActive))
    (Variables|Default|SetTaskActive true)
    (Variables|Default|SetTaskEndTime (+ (Utilities|Time|GetGameTimeinSeconds) (Class|BTFunctionLibrary|GetBlackboardValueasFloat (Variables|Default|GetCircleDuration))))))