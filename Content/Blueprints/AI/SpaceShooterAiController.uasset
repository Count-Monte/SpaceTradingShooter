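; AI controller for ships in a space shooter, driven by the BT_AI_Ship behavior tree.
; On BeginPlay it loads the BB_AI_Ship blackboard, writes the circle and assault durations into it and starts the tree.
; Possess and Tick are empty.
; Disconnected nodes hold an unused hand-coded version of faction-based targeting, orbit or assault steering, firing and debug arrows.
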(event EventBeginPlay
  (bind _blackboardcomponent (Class|AIController|UseBlackboard "/Game/Blueprints/AI/BB_AI_Ship.BB_AI_Ship"))
  (AI|Components|Blackboard|SetValueasFloat _blackboardcomponent (Variables|Default|GetCircleDurationKey) (Variables|Default|GetCircleDuration))
  (AI|Components|Blackboard|SetValueasFloat _blackboardcomponent (Variables|Default|GetAssaultDurationKey) (Variables|Default|GetAssaultDuration))
  (AI|RunBehaviorTree "/Game/Blueprints/AI/BT_AI_Ship.BT_AI_Ship"))

(event EventTick
  (params (DeltaSeconds :type Float%20%28single-precision%29)))

(event EventPossess
  (params (PossessedPawn :type Pawn%20Object%20Reference)))

(fn ConstructionScript)