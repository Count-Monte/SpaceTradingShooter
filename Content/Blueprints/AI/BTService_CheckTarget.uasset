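; Behavior tree service that keeps the Target and HasTarget blackboard values up to date for an AI-controlled Ship.
; Each tick it keeps a valid existing target without rechecking range, and otherwise takes the first actor returned by the ship's GetActorsInRangeOfSensor.
; If none is found or the pawn is not a Ship, it clears HasTarget but leaves Target untouched.
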(event EventReceiveTickAI
  (params (OwnerController :type AI%20Controller%20Object%20Reference) (ControlledPawn :type Pawn%20Object%20Reference) (DeltaSeconds :type Float%20%28single-precision%29))
  (bind _hastarget (Variables|Default|GetHasTarget))
  (if (Class|BTFunctionLibrary|GetBlackboardValueasBool _hastarget)
    (Utilities|IsValid (Class|BTFunctionLibrary|GetBlackboardValueasObject (Variables|Default|GetTarget))
      (:Is%20Not%20Valid
        _)))
  (bind _asship (Utilities|Casting|CastToShip ControlledPawn)
    (:then
      (bind _ships (Default|GetActorsinRangeOfSensor _asship))
      (if (> (Utilities|Array|Length _ships) 0)
        (Class|BTFunctionLibrary|SetBlackboardValueasBool _hastarget true)
        (Class|BTFunctionLibrary|SetBlackboardValueasObject (Variables|Default|GetTarget) (Utilities|Array|Get(acopy) _ships))
        (else
          (Class|BTFunctionLibrary|SetBlackboardValueasBool _hastarget false :!label _label))))
    (:CastFailed
      (goto _label))))